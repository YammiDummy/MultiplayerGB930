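; BP_MultiGameMode is a multiplayer game mode that sorts joining players into two balanced teams.
; PostLogin adds each BP_MultiPlayerController to the smaller team array, Team 1 on ties, setting its team ID and a count-based name.
; Logout routes through a custom event that looks up the controller by team ID, removing it only when its found index is zero, then prints both team counts.
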(event `self.K2_PostLogin`
  (params (NewPlayer :type "PlayerController Object Reference"))
  (bind _asbp_multi_player_controller (cast `/Game/MyContent/BP/BP_MultiPlayerController` NewPlayer)
    (:`then`
      (if (> (`KismetArrayLibrary.Array_Length` (`self.Team 1`)) (`KismetArrayLibrary.Array_Length` (`self.Team 2`)))
        (`KismetArrayLibrary.Array_Add` (`self.Team 2`) _asbp_multi_player_controller)
        (`/Game/MyContent/BP/BP_MultiPlayerController.SetTeamID` _asbp_multi_player_controller 2)
        (set `/Game/MyContent/BP/BP_MultiPlayerController.Player Name` (`KismetStringLibrary.Concat_StrStr` "Team2_" "Player" (`KismetStringLibrary.Conv_IntToString` (`KismetArrayLibrary.Array_Length` (`self.Team 2`)))) _asbp_multi_player_controller)
        (else
          (`KismetArrayLibrary.Array_Add` (`self.Team 1`) _asbp_multi_player_controller)
          (`/Game/MyContent/BP/BP_MultiPlayerController.SetTeamID` _asbp_multi_player_controller 1)
          (set `/Game/MyContent/BP/BP_MultiPlayerController.Player Name` (`KismetStringLibrary.Concat_StrStr` "Team1_" "Player" (`KismetStringLibrary.Conv_IntToString` (`KismetArrayLibrary.Array_Length` (`self.Team 1`)))) _asbp_multi_player_controller))))
    (:`CastFailed`
      (`KismetSystemLibrary.PrintString` "Login to server failed!"))))

(event `self.K2_OnLogout`
  (params (ExitingController :type "Controller Object Reference"))
  (`KismetSystemLibrary.PrintString` "Hello")
  (`self.Server_LogOut` (cast `/Game/MyContent/BP/BP_MultiPlayerController` ExitingController :!pure true)))

(event `Server_LogOut`
  (params (NewParam :type "/Game/MyContent/BP/BP_MultiPlayerController Object Reference"))
  (bind _team_1 (`self.Team 1`))
  (bind _team_id (`/Game/MyContent/BP/BP_MultiPlayerController.Team ID` NewParam))
  (bind _team_2 (`self.Team 2`))
  (bind _returnvalue (`KismetArrayLibrary.Array_Find` _team_1 NewParam))
  (bind _returnvalue_2 (`KismetArrayLibrary.Array_Find` _team_2 NewParam))
  (if (== _team_id 1)
    (if (not (`KismetMathLibrary.Conv_IntToBool` _returnvalue))
      (`KismetArrayLibrary.Array_Remove` _team_1 _returnvalue)
      (`self.Server_Print`))
    (elif (== _team_id 2)
      (if (not (`KismetMathLibrary.Conv_IntToBool` _returnvalue_2))
        (`KismetArrayLibrary.Array_Remove` _team_2 _returnvalue_2)
        (`self.Server_Print`))
      (else
        (`KismetSystemLibrary.PrintString` "Player Controller has no Team ID")))))

(event `Server_Print`
  (`KismetSystemLibrary.PrintString` (`KismetStringLibrary.Concat_StrStr` "Team 1 Players: " (`KismetStringLibrary.Conv_IntToString` (`KismetArrayLibrary.Array_Length` (`self.Team 1`))) "Team 2 Players: " (`KismetStringLibrary.Conv_IntToString` (`KismetArrayLibrary.Array_Length` (`self.Team 2`))))))

(fn `UserConstructionScript`)