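; BP_HealthComponent is an actor component that tracks its owner's health and destroys the owner when damage would bring health to zero or below.
; CurrentHealth starts at MaxHealth and is reduced by the TakeDamage event.
; A RepNotify on CurrentHealth calls UpdateHealthBar, which sets the health percentage on the WBP_HealthBar widget of an owning BP_MultiCharacter.
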(event `self.ReceiveBeginPlay`
  (set `self.Current Health` (`self.Max Health`)))

(event `Take Damage`
  (params (`Damage Taken` :type "Float (double-precision)"))
  (bind _returnvalue (- (`self.Current Health`) `Damage Taken`))
  (if (> _returnvalue 0.0)
    (set `self.Current Health` _returnvalue)
    (else
      (`Actor.K2_DestroyActor` (`self.GetOwner`)))))

(event `Update Health Bar`
  (bind _asbp_multi_character (cast `/Game/MyContent/BP/BP_MultiCharacter` (`self.GetOwner`)))
  (bind _aswbp_health_bar (cast `/Game/MyContent/UI/WBP_HealthBar` (`WidgetComponent.GetWidget` (`/Game/MyContent/BP/BP_MultiCharacter.HealthBar` _asbp_multi_character))))
  (`ProgressBar.SetPercent` (`/Game/MyContent/UI/WBP_HealthBar.HealthProgress` _aswbp_health_bar) (/ (`self.Current Health`) (`self.Max Health`))))

(fn `OnRep_Current Health`
  (`self.Update Health Bar`))