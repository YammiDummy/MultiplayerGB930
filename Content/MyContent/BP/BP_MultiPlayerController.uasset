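; BP_MultiPlayerController is a multiplayer player controller that stores a team ID and handles player removal.
; SetTeamID forwards the ID to a server event that saves it.
; Q sends the controlled pawn to a server destroy event and calls RemovePlayer on itself, which the server event repeats through DestroyController.
; T casts the game mode to BP_MultiGameMode and calls its ServerPrint.
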(event `SetTeamID`
  (params (`Team ID` :type Byte))
  (`self.Server_SetTeamID` `Team ID`))

(event `Server_SetTeamID`
  (params (`Team ID` :type Byte))
  (set `self.Team ID` `Team ID`))

(event `Key|Q`
  (params (Key :type "Key Structure"))
  (:`Pressed`
    (`self.Server_DestroyActor` (`self.K2_GetPawn` self))
    (`GameplayStatics.RemovePlayer` self)))

(event `Server_DestroyActor`
  (params (`Player Pawn` :type "Pawn Object Reference"))
  (`self.K2_DestroyActor` `Player Pawn`)
  (`self.DestroyController`))

(event `DestroyController`
  (`GameplayStatics.RemovePlayer` self))

(event `Key|T`
  (params (Key :type "Key Structure"))
  (:`Pressed`
    (bind _asbp_multi_game_mode (cast `/Game/MyContent/BP/BP_MultiGameMode` (`GameplayStatics.GetGameMode`)))
    (`/Game/MyContent/BP/BP_MultiGameMode.Server_Print` _asbp_multi_game_mode)))

(fn `UserConstructionScript`)