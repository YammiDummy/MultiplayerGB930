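; Networked projectile that damages multiplayer characters it overlaps and expires after a set lifetime.
; The server moves it forward each Tick by setting its location without sweep, rather than using a movement component.
; Server-handled sphere overlaps ignore the owner, damage BP_MultiCharacter with a multicast explosion effect, and also end the projectile on contact with another projectile.
; Both impacts and timer expiry destroy it through a short server-side delay.
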(event `self.ReceiveBeginPlay`
  (`KismetSystemLibrary.K2_SetTimerDelegate` (delegate `Lifetime end`) (`self.Lifetime`)))

(event `Lifetime end`
  (`self.Server_LifetimeEnd`))

(event `Server_LifetimeEnd`
  (`KismetSystemLibrary.Delay` 0.2)
  (`self.K2_DestroyActor`))

(event `Server_Move`
  (params (`Delta Time` :type "Float (double-precision)"))
  (`self.K2_SetActorLocation` (+ (* (`self.GetActorForwardVector`) (* `Delta Time` (`self.Speed`))) (`self.K2_GetActorLocation`))))

(event `self.ReceiveTick`
  (params (DeltaSeconds :type "Float (single-precision)"))
  (if (`KismetSystemLibrary.IsServer`)
    (`self.Server_Move` DeltaSeconds)))

(event `self.SphereRoot.OnComponentBeginOverlap`
  (params (OverlappedComponent :type "PrimitiveComponent Object Reference") (OtherActor :type "Actor Object Reference") (OtherComp :type "PrimitiveComponent Object Reference") (OtherBodyIndex :type Integer) (bFromSweep :type Boolean) (SweepResult :type "HitResult Structure (by ref)"))
  (if (`KismetSystemLibrary.IsServer`)
    (`self.Server_Collision` OtherActor (`self.K2_GetActorLocation`))))

(event `Server_Collision`
  (params (OtherActor :type "Actor Object Reference") (Location :type "Vector Structure"))
  (if (!= OtherActor (`self.GetOwner`))
    (bind _asbp_multi_character (cast `/Game/MyContent/BP/BP_MultiCharacter` OtherActor)
      (:`then`
        (`/Game/MyContent/BP/BP_MultiCharacter.TakeDamage` _asbp_multi_character (`self.Damage`))
        (`self.Multicast_HitEffect` Location)
        (`self.Server_LifetimeEnd`))
      (:`CastFailed`
        (cast `/Game/MyContent/BP/BP_Projectile` OtherActor)
        (if (!= OtherActor self)
          (`self.Server_LifetimeEnd`))))))

(event `SpawnHitEffect`
  (params (`Hit Location` :type "Vector Structure"))
  (`GameplayStatics.SpawnEmitterAtLocation` "/Game/StarterContent/Particles/P_Explosion.P_Explosion" `Hit Location`))

(event `Multicast_HitEffect`
  (params (`Hit Location` :type "Vector Structure"))
  (`self.SpawnHitEffect` `Hit Location`))

(fn `UserConstructionScript`)